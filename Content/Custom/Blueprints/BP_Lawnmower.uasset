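; BP_Lawnmower is a one-shot lawnmower that travels along a spline once a BP_Nut touches its trigger.
; The Sphere's begin overlap accepts only a static mesh component on a BP_Nut, passes through a DoOnce, and starts a Timeline after a short delay.
; The Timeline maps its track value to distance along the Spline and sets the Cube's world location there without sweeping, leaving rotation untouched.
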(event `self.Sphere.OnComponentBeginOverlap`
  (params (OverlappedComponent :type "PrimitiveComponent Object Reference") (OtherActor :type "Actor Object Reference") (OtherComp :type "PrimitiveComponent Object Reference") (OtherBodyIndex :type Integer) (bFromSweep :type Boolean) (SweepResult :type "HitResult Structure (by ref)"))
  (bind _spline (`self.Spline`))
  (cast `StaticMeshComponent` OtherComp)
  (cast `/Game/Custom/Blueprints/BP_Nut` OtherActor)
  (`/Engine/EditorBlueprintResources/StandardMacros.DoOnce` false
    (:`Completed`
      (`KismetSystemLibrary.Delay` 0.2)
      (bind (_direction _newtrack_0) (`Timeline|Timeline` :!via `PlayFromStart`)
        (:`Update`
          (`SceneComponent.K2_SetWorldLocation` (`self.Cube`) (`SplineComponent.GetLocationAtDistanceAlongSpline` _spline (`KismetMathLibrary.Lerp` 0.0 (`SplineComponent.GetSplineLength` _spline) _newtrack_0) "World") false false))))))

(fn `UserConstructionScript`)