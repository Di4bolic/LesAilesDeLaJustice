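; Trigger volume that ends the game when a falling battery enters it and causes an electrocution.
; The Box overlap filters for BP_FallingBattery and fires once, spawning the NS_Eclair Niagara effect and a sound at the Elec component.
; After a delay it adds the WBP_EndScreen widget to the viewport and shows the mouse cursor.
; The construction script positions Elec from the POSELEC variable.
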(event `self.Box.OnComponentBeginOverlap`
  (params (OverlappedComponent :type "PrimitiveComponent Object Reference") (OtherActor :type "Actor Object Reference") (OtherComp :type "PrimitiveComponent Object Reference") (OtherBodyIndex :type Integer) (bFromSweep :type Boolean) (SweepResult :type "HitResult Structure (by ref)"))
  (bind _returnvalue (`GameplayStatics.GetPlayerController` 0))
  (bind _returnvalue_2 (`SceneComponent.K2_GetComponentLocation` (`self.elec`)))
  (cast `/Game/Custom/Blueprints/BP_FallingBattery` OtherActor)
  (`/Engine/EditorBlueprintResources/StandardMacros.DoOnce` false
    (:`Completed`
      (`NiagaraFunctionLibrary.SpawnSystemAtLocation` "/Game/Custom/VFX/NS_Eclair.NS_Eclair" _returnvalue_2 (struct) (1.0 1.0 1.0) true true "AutoRelease")
      (`GameplayStatics.PlaySoundAtLocation` "/Game/StarterContent/Audio/Light02.Light02" _returnvalue_2 (struct) 1.0 1.0 0.0 null null null null)
      (`KismetSystemLibrary.Delay` 5.0)
      (bind _returnvalue_3 (`|CreateWidget` "/Game/Custom/Blueprints/WBP_EndScreen.WBP_EndScreen_C" _returnvalue))
      (`UserWidget.AddToViewport` _returnvalue_3 0)
      (set `PlayerController.bShowMouseCursor` true _returnvalue))))

(fn `UserConstructionScript`
  (`SceneComponent.K2_SetRelativeLocation` (`self.elec`) (`self.POS ELEC`) false false))