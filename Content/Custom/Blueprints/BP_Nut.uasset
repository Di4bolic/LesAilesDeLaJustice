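; BP_Nut is a nut actor that stays pinned in place until it gets blown.
; BeginPlay records the mesh's world location, and each Tick zeroes its physics linear velocity and resets it to that location while Blowed is false.
; GetBlowed sets Blowed once through a DoOnce and prints a debug message, after which the mesh is no longer held.
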(event `self.ReceiveBeginPlay`
  (set `self.OgLocation` (`SceneComponent.K2_GetComponentLocation` (`self.Mesh`))))

(event `self.ReceiveTick`
  (params (DeltaSeconds :type "Float (single-precision)"))
  (bind _mesh (`self.Mesh`))
  (if (not (`self.Blowed`))
    (`PrimitiveComponent.SetAllPhysicsLinearVelocity` _mesh (0.0 0.0 0.0) false)
    (`SceneComponent.K2_SetWorldLocation` _mesh (`self.OgLocation`) false false)))

(event `GetBlowed`
  (`/Engine/EditorBlueprintResources/StandardMacros.DoOnce` false
    (:`Completed`
      (set `self.Blowed` true)
      (`KismetSystemLibrary.PrintString` "Hello"))))

(fn `UserConstructionScript`)