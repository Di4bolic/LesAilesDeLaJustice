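; Fertilizer sachet actor that topples on a Fall event and spills transportable fertilizer pieces once it comes to rest.
; Fall shoves the Book component along its right vector with a large impulse, then polls its velocity on short delays until it reaches zero.
; It then spawns a batch of BP_Transportable actors at SeedSpawnPoint, each given a sphere mesh and tagged as Fertilizer.
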(event `Fall`
  (bind _returnvalue_location (`KismetMathLibrary.BreakTransform` (`SceneComponent.K2_GetComponentToWorld` (`self.SeedSpawnPoint`))))
  (`PrimitiveComponent.AddImpulse` (`self.Book`) (* (`SceneComponent.GetRightVector` (`self.Book`)) 99999.0) "None" false)
  (`KismetSystemLibrary.Delay` 1.0)
  (if (== (`SceneComponent.GetComponentVelocity` (`self.Book`)) (0.0 0.0 0.0)) :!label _label
    (for _ (range 10)
      (bind _returnvalue (`|SpawnActorFromClass` "/Game/Custom/Blueprints/BP_Transportable.BP_Transportable_C" (`KismetMathLibrary.MakeTransform` _returnvalue_location) "Undefined" "MultiplyWithRoot" null null))
      (`StaticMeshComponent.SetStaticMesh` (`/Game/Custom/Blueprints/BP_Transportable.Mesh` _returnvalue) "/Game/StarterContent/Shapes/Shape_Sphere.Shape_Sphere")
      (set `/Game/Custom/Blueprints/BP_Transportable.Tag` "Fertilizer" _returnvalue))
    (else
      (`KismetSystemLibrary.Delay` 0.1)
      (goto _label))))

(fn `UserConstructionScript`)