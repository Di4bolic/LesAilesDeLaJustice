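; BP_GrowingPlant is a plant that grows once when fed fertilizer, then produces a BP_Nut.
; A sphere overlap with a static mesh of a BP_Transportable tagged "Fertilizer" destroys that item and plays the NS_Growing effect.
; A half-speed Timeline scales the plant up with growth and stretch curves, making it proportionally taller and narrower.
; After a short delay the nut spawns at SeedSpawnPoint, which the construction script positions from SeedPos.
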(event `self.ReceiveBeginPlay`
  (`TimelineComponent.SetPlayRate` (`self.Timeline`) 0.5))

(event `self.SphereCollision.OnComponentBeginOverlap`
  (params (OverlappedComponent :type "PrimitiveComponent Object Reference") (OtherActor :type "Actor Object Reference") (OtherComp :type "PrimitiveComponent Object Reference") (OtherBodyIndex :type Integer) (bFromSweep :type Boolean) (SweepResult :type "HitResult Structure (by ref)"))
  (cast `StaticMeshComponent` OtherComp)
  (bind _asbp_transportable (cast `/Game/Custom/Blueprints/BP_Transportable` OtherActor))
  (if (`KismetStringLibrary.EqualEqual_StrStr` (`/Game/Custom/Blueprints/BP_Transportable.Tag` _asbp_transportable) "Fertilizer")
    (`/Engine/EditorBlueprintResources/StandardMacros.DoOnce` false
      (:`Completed`
        (`self.K2_DestroyActor` _asbp_transportable)
        (`NiagaraFunctionLibrary.SpawnSystemAtLocation` "/Game/Custom/VFX/NS_Growing.NS_Growing" (`SceneComponent.K2_GetComponentLocation` (`self.Plant`)))
        (bind (_direction _plantgrowth _plantstretch) (`Timeline|Timeline` :!via `PlayFromStart`)
          (:`Update`
            (bind _returnvalue (`KismetMathLibrary.Lerp` 1.0 0.7 _plantstretch))
            (`SceneComponent.SetWorldScale3D` (`self.Plant`) (* (`KismetMathLibrary.Lerp` 1.0 10.0 _plantgrowth) (`KismetMathLibrary.MakeVector` _returnvalue _returnvalue (`KismetMathLibrary.Lerp` 1.0 1.5 _plantstretch)))))
          (:`Finished`
            (`KismetSystemLibrary.Delay` 1.0)
            (`|SpawnActorFromClass` "/Game/Custom/Blueprints/BP_Nut.BP_Nut_C" (`KismetMathLibrary.MakeTransform` (`SceneComponent.K2_GetComponentLocation` (`self.SeedSpawnPoint`))) "Undefined" "MultiplyWithRoot" null null)))))))

(fn `UserConstructionScript`
  (`SceneComponent.K2_SetRelativeLocation` (`self.SeedSpawnPoint`) (`self.SeedPos`) false false))