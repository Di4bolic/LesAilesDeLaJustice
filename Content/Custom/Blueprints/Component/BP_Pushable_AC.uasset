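; BP_Pushable_AC is a component that lets its owning actor's static mesh be pushed as a physics object.
; On BeginPlay it raises the mesh's mass to a very high override if it is lighter.
; GetPushed enables physics simulation when it is off, then applies the incoming impulse, scaled by a large constant to suit that mass, at the given location.
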(event `self.ReceiveBeginPlay`
  (bind _returnvalue (`Actor.GetComponentByClass` (`self.GetOwner`) "/Script/Engine.StaticMeshComponent"))
  (if (< (`PrimitiveComponent.GetMass` _returnvalue) 99999.0)
    (`PrimitiveComponent.SetMassOverrideInKg` _returnvalue "None" 99999.0 true)))

(event `GetPushed`
  (params (Impulse :type "Vector Structure") (Location :type "Vector Structure"))
  (bind _returnvalue (`Actor.GetComponentByClass` (`self.GetOwner`) "/Script/Engine.StaticMeshComponent"))
  (if (not (`SceneComponent.IsSimulatingPhysics` _returnvalue "None"))
    (`PrimitiveComponent.SetSimulatePhysics` _returnvalue true))
  (`PrimitiveComponent.AddImpulseAtLocation` _returnvalue (* Impulse 40000000.0) Location "None"))