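; BP_FieldStress is a field system actor that breaks and scatters Chaos physics objects within a sphere when play begins.
; On BeginPlay it applies a strong external cluster strain through a radial falloff sized and centered on its Sphere component.
; It then applies an outward radial linear velocity, culled by a matching radial falloff.
; Tick, overlap and construction logic are empty.
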(event `self.ReceiveBeginPlay`
  (bind _sphere (`self.Sphere`))
  (bind _returnvalue (`SceneComponent.K2_GetComponentLocation` _sphere))
  (bind _returnvalue_2 (`RadialFalloff.SetRadialFalloff` (`self.RadialFalloff`) 1000000.0 0.0 1.0 0.0 (`SphereComponent.GetScaledSphereRadius` _sphere) _returnvalue "Field_FallOff_None"))
  (`FieldSystemComponent.ApplyPhysicsField` (`self.FieldSystemComponent`) true "Field_ExternalClusterStrain" null _returnvalue_2)
  (`FieldSystemComponent.ApplyPhysicsField` (`self.FieldSystemComponent`) true "Field_LinearVelocity" null (`CullingField.SetCullingField` (`self.CullingField`) _returnvalue_2 (`RadialVector.SetRadialVector` (`self.RadialVector`) 1000.0 _returnvalue) "Field_Culling_Inside")))

(event `self.ReceiveTick`
  (params (DeltaSeconds :type "Float (single-precision)")))

(fn `UserConstructionScript`)