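; BP_Transportable is a transportable item whose Tag selects its look, with variants for Mentos, Cigarette and Fertilizer.
; SetMeshWithTag sets mesh, material and scale per tag, running in both the construction script and BeginPlay, which also attaches smoke to cigarettes.
; Its collision overlap sets itself as the third-person character's TransportableObjectInRange, clearing that on exit only if it is still the current one.
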(event `self.ReceiveBeginPlay`
  (`self.SetMeshWithTag`)
  (if (`KismetStringLibrary.EqualEqual_StrStr` (`self.Tag`) "Cigarette")
    (`GameplayStatics.SpawnEmitterAttached` "/Game/StarterContent/Particles/P_Smoke.P_Smoke" (`self.Mesh`) "None" (0.0 10.0 0.0) (struct) (0.1 0.1 0.1))))

(event `SetMeshWithTag`
  (bind _mesh (`self.Mesh`))
  (bind _collision (`self.Collision`))
  (switch `string` (`self.Tag`)
    (:`Default`
      (`StaticMeshComponent.SetStaticMesh` _mesh "/Game/StarterContent/Props/MaterialSphere.MaterialSphere"))
    (:`Mentos`
      (`StaticMeshComponent.SetStaticMesh` _mesh "/Game/StarterContent/Props/MaterialSphere.MaterialSphere")
      (`SceneComponent.SetRelativeScale3D` _mesh (0.5 0.5 0.25))
      (`SceneComponent.SetWorldScale3D` _collision (1.0 1.0 1.0)))
    (:`Cigarette`
      (`StaticMeshComponent.SetStaticMesh` _mesh "/Game/Custom/Meshes/Cigarette/SM_Cigarette.SM_Cigarette")
      (`SceneComponent.SetRelativeScale3D` _mesh (4.0 4.0 4.0))
      (`SceneComponent.SetWorldScale3D` _collision (1.0 1.0 1.0)))
    (:`Fertilizer`
      (`StaticMeshComponent.SetStaticMesh` _mesh "/Game/StarterContent/Props/MaterialSphere.MaterialSphere")
      (`PrimitiveComponent.SetMaterial` _mesh 0 "/Game/StarterContent/Materials/M_Wood_Walnut.M_Wood_Walnut")
      (`SceneComponent.SetRelativeScale3D` _mesh (0.5 0.5 0.5)))))

(event `self.Collision.OnComponentBeginOverlap`
  (params (OverlappedComponent :type "PrimitiveComponent Object Reference") (OtherActor :type "Actor Object Reference") (OtherComp :type "PrimitiveComponent Object Reference") (OtherBodyIndex :type Integer) (bFromSweep :type Boolean) (SweepResult :type "HitResult Structure (by ref)"))
  (bind _asbp_third_person_character (cast `/Game/ThirdPerson/Blueprints/BP_ThirdPersonCharacter` OtherActor))
  (set `/Game/ThirdPerson/Blueprints/BP_ThirdPersonCharacter.TransportableObjectInRange` self _asbp_third_person_character))

(event `self.Collision.OnComponentEndOverlap`
  (params (OverlappedComponent :type "PrimitiveComponent Object Reference") (OtherActor :type "Actor Object Reference") (OtherComp :type "PrimitiveComponent Object Reference") (OtherBodyIndex :type Integer))
  (bind _asbp_third_person_character (cast `/Game/ThirdPerson/Blueprints/BP_ThirdPersonCharacter` OtherActor))
  (if (== (`/Game/ThirdPerson/Blueprints/BP_ThirdPersonCharacter.TransportableObjectInRange` _asbp_third_person_character) self)
    (set `/Game/ThirdPerson/Blueprints/BP_ThirdPersonCharacter.TransportableObjectInRange` null _asbp_third_person_character)))

(fn `UserConstructionScript`
  (`self.SetMeshWithTag`))