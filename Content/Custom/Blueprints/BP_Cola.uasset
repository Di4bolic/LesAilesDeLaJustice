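; BP_Cola is a cola prop that reacts explosively, one time only, when Mentos is dropped into it.
; Its collision sphere detects a static mesh component of a BP_Transportable tagged "Mentos", destroys that actor and spawns a Niagara drop effect at VFXLocation.
; After a short delay, a large explosion particle effect and sound play at the mesh, which stays in place.
; The construction script positions VFXLocation from the VFXPos variable.
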(event `self.ReceiveBeginPlay`)

(event `self.SphereCollision.OnComponentBeginOverlap`
  (params (OverlappedComponent :type "PrimitiveComponent Object Reference") (OtherActor :type "Actor Object Reference") (OtherComp :type "PrimitiveComponent Object Reference") (OtherBodyIndex :type Integer) (bFromSweep :type Boolean) (SweepResult :type "HitResult Structure (by ref)"))
  (bind _returnvalue (`SceneComponent.K2_GetComponentLocation` (`self.Mesh`)))
  (cast `StaticMeshComponent` OtherComp)
  (bind _asbp_transportable (cast `/Game/Custom/Blueprints/BP_Transportable` OtherActor))
  (if (`KismetStringLibrary.EqualEqual_StrStr` (`/Game/Custom/Blueprints/BP_Transportable.Tag` _asbp_transportable) "Mentos")
    (`/Engine/EditorBlueprintResources/StandardMacros.DoOnce` false
      (:`Completed`
        (`self.K2_DestroyActor` _asbp_transportable)
        (`NiagaraFunctionLibrary.SpawnSystemAtLocation` "/Game/Custom/VFX/NS_MentosDrop.NS_MentosDrop" (`SceneComponent.K2_GetComponentLocation` (`self.VFXLocation`)))
        (`KismetSystemLibrary.Delay` 2.0)
        (`GameplayStatics.SpawnEmitterAtLocation` "/Game/StarterContent/Particles/P_Explosion.P_Explosion" _returnvalue (struct) (25.0 25.0 25.0))
        (`GameplayStatics.PlaySoundAtLocation` "/Game/StarterContent/Audio/Explosion01.Explosion01" _returnvalue (struct) 1.0 1.0 0.0 null null null null)))))

(fn `UserConstructionScript`
  (`SceneComponent.K2_SetRelativeLocation` (`self.VFXLocation`) (`self.VFXPos`) false false))