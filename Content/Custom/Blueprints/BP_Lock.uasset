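; BP_Lock is a door lock that is triggered when a BP_FallingFlowerPot overlaps its box.
; The overlap fires a one-shot Fly event, where a timeline moves Cube2 along a spline with matching pitch and offset yaw, paced by Speed.
; When the flight finishes, the three cube components are destroyed and a second timeline swings the referenced Door open by rotating its yaw.
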(event `self.ReceiveBeginPlay`
  (`TimelineComponent.SetPlayRate` (`self.Timeline`) (/ 1.0 (`self.Speed`))))

(event `self.Box.OnComponentBeginOverlap`
  (params (OverlappedComponent :type "PrimitiveComponent Object Reference") (OtherActor :type "Actor Object Reference") (OtherComp :type "PrimitiveComponent Object Reference") (OtherBodyIndex :type Integer) (bFromSweep :type Boolean) (SweepResult :type "HitResult Structure (by ref)"))
  (cast `/Game/Custom/Blueprints/BP_FallingFlowerPot` OtherActor)
  (`self.Fly`))

(event `Fly`
  (bind _spline (`self.Spline`))
  (bind _cube2 (`self.Cube2`))
  (bind _zrot (`self.ZRot`))
  (bind (_returnvalue_roll _returnvalue_pitch _returnvalue_yaw) (`KismetMathLibrary.BreakRotator` (`self.K2_GetActorRotation` (`self.Door`))))
  (`/Engine/EditorBlueprintResources/StandardMacros.DoOnce` false
    (:`Completed`
      (bind (_direction _newtrack_0) (`Timeline|Timeline` :!via `PlayFromStart`)
        (:`Update`
          (bind _returnvalue (`KismetMathLibrary.Lerp` 0.0 (`SplineComponent.GetSplineLength` _spline) _newtrack_0))
          (`SceneComponent.K2_SetWorldLocation` _cube2 (`SplineComponent.GetLocationAtDistanceAlongSpline` _spline _returnvalue "World") false false)
          (bind (_returnvalue_roll_2 _returnvalue_pitch_2 _returnvalue_yaw_2) (`KismetMathLibrary.BreakRotator` (`SplineComponent.GetRotationAtDistanceAlongSpline` _spline _returnvalue "Local")))
          (`SceneComponent.K2_SetWorldRotation` _cube2 (`KismetMathLibrary.MakeRotator` 0.0 _returnvalue_pitch_2 (+ _returnvalue_yaw_2 (`self.Correction`))) false false))
        (:`Finished`
          (`ActorComponent.K2_DestroyComponent` (`self.Cube`))
          (`ActorComponent.K2_DestroyComponent` (`self.Cube1`))
          (`ActorComponent.K2_DestroyComponent` (`self.Cube2`))
          (set `self.ZRot` _returnvalue_yaw)
          (bind (_direction_2 _newtrack_0_2) (`Timeline|Timeline_0` :!via `PlayFromStart`)
            (:`Update`
              (`self.K2_SetActorRotation` (`self.Door`) (`KismetMathLibrary.RLerp` (`KismetMathLibrary.MakeRotator` 0.0 0.0 _zrot) (`KismetMathLibrary.MakeRotator` 0.0 0.0 (+ _zrot -60.0)) _newtrack_0_2) false))))))))

(fn `UserConstructionScript`)