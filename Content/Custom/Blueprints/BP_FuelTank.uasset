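; BP_FuelTank is a fuel tank actor that tips over shortly after play begins and spreads a fuel puddle.
; A one-shot timeline rolls the mesh while scaling the puddle, whose position is set in the construction script from PuddlePos.
; Its flammable zone counts overlapping BP_Transportable meshes tagged as cigarettes.
; A separate one-shot SetFire event, not called within this graph, spawns a large fire emitter at that zone.
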(event `self.ReceiveBeginPlay`
  (`KismetSystemLibrary.Delay` 1.0)
  (`self.FlipTheTank`))

(event `self.ImflamableZone.OnComponentBeginOverlap`
  (params (OverlappedComponent :type "PrimitiveComponent Object Reference") (OtherActor :type "Actor Object Reference") (OtherComp :type "PrimitiveComponent Object Reference") (OtherBodyIndex :type Integer) (bFromSweep :type Boolean) (SweepResult :type "HitResult Structure (by ref)"))
  (cast `StaticMeshComponent` OtherComp)
  (bind _asbp_transportable (cast `/Game/Custom/Blueprints/BP_Transportable` OtherActor))
  (if (`KismetStringLibrary.EqualEqual_StrStr` (`/Game/Custom/Blueprints/BP_Transportable.Tag` _asbp_transportable) "Cigarette")
    (`/Engine/EditorBlueprintResources/StandardMacros.IncrementInt` (`self.Cigarette`))))

(event `FlipTheTank`
  (bind _puddle (`self.Puddle`))
  ;[0.2969 0.2969 0.2969] Anim
  (`/Engine/EditorBlueprintResources/StandardMacros.DoOnce` false
    (:`Completed`
      (`TimelineComponent.SetPlayRate` (`self.Timeline`) 1.5)
      (bind (_direction _tank _puddle_2) (`Timeline|Timeline` :!via `PlayFromStart`)
        (:`Update`
          (`SceneComponent.K2_SetRelativeRotation` (`self.Mesh`) (`KismetMathLibrary.MakeRotator` (* _tank 90.0) 0.0 -90.0) false false)
          (bind _returnvalue (* _puddle_2 5.0))
          (`SceneComponent.SetRelativeScale3D` _puddle (`KismetMathLibrary.MakeVector` _returnvalue _returnvalue 1.0))
          (bind _returnvalue_2 (!= _puddle_2 0.0))
          (if _returnvalue_2
            (`/Engine/EditorBlueprintResources/StandardMacros.DoOnce` false
              (:`Completed`
                (`SceneComponent.SetVisibility` _puddle _returnvalue_2 false)))))))))

(event `SetFire`
  ;[0.2969 0.2969 0.2969] Fire
  (`/Engine/EditorBlueprintResources/StandardMacros.DoOnce` false
    (:`Completed`
      (`GameplayStatics.SpawnEmitterAtLocation` "/Game/StarterContent/Particles/P_Fire.P_Fire" (`SceneComponent.K2_GetComponentLocation` (`self.ImflamableZone`)) (struct) (20.0 20.0 20.0)))))

(fn `UserConstructionScript`
  (`SceneComponent.K2_SetRelativeLocation` (`self.Puddle`) (`self.PuddlePos`) false false)
  (`SceneComponent.K2_SetRelativeLocation` (`self.ImflamableZone`) (0.0 0.0 0.0) false false))